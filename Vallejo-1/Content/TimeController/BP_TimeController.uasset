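; BP_TimeController is a Blueprint that controls the date and time of day of a SunSky.
; Custom events set the Month and Day, converting the input to an integer and calling UpdateSun after each change.
; SetTimeOfDay writes SolarTime directly without calling UpdateSun.
; It has no active BeginPlay or Tick logic, so changes happen only when these events are called.
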(event Custom|SetMonth
  (params (SetMonth :type Boolean))
  (bind _sunsky (Variables|Default|GetSunSky))
  (Variables|/SunPosition/SunSky.SunSky_C|SetMonth _sunsky (Math|Conversions|ToInteger(Boolean) SetMonth))
  (Default|UpdateSun _sunsky))

(event Custom|SetDay
  (params (Set%20Day :type Boolean))
  (bind _sunsky (Variables|Default|GetSunSky))
  (Variables|/SunPosition/SunSky.SunSky_C|SetDay _sunsky (Math|Conversions|ToInteger(Boolean) Set%20Day))
  (Default|UpdateSun _sunsky))

(event Custom|SetTimeOfDay
  (params (NewTime :type Float%20%28double-precision%29))
  (Variables|/SunPosition/SunSky.SunSky_C|SetSolarTime (Variables|Default|GetSunSky) NewTime))

(event EventBeginPlay)

(event Collision|EventActorBeginOverlap
  (params (OtherActor :type Actor%20Object%20Reference)))

(event EventTick
  (params (DeltaSeconds :type Float%20%28single-precision%29)))

(fn ConstructionScript)